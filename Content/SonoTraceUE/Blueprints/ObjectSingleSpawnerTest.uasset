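; A test spawner actor for SonoTraceUE that periodically replaces a single randomly placed static mesh component on itself.
; At a set rate on Tick, it destroys the previous component and adds one with random offset, rotation and scale.
; It unregisters and re-registers itself with every SonoTraceUEActor found at BeginPlay around each swap.
; Ticking stops once the spawn count reaches its maximum.
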(event EventTick
  (params (DeltaSeconds :type Float%20%28single-precision%29))
  (bind _spawnradius (Variables|Default|GetSpawnRadius))
  (bind _returnvalue (* _spawnradius -1.0))
  (bind _output_get (Variables|Default|SetTimePassed (+ DeltaSeconds (Variables|Default|GetTimePassed))))
  (if (>= _output_get (/ 1.0 (Variables|Default|GetSpawnRate)))
    (Variables|Default|SetTimePassed 0.0)
    (Utilities|IsValid (Variables|Default|GetStaticComponentReference)
      (:Is%20Valid
        (for _array_element (Variables|Default|GetSonoTraceUEActors)
          (Class|SonoTraceUEActor|RemoveActor _array_element self))
        (Components|DestroyComponent (Variables|Default|GetStaticComponentReference)))
      (:Is%20Not%20Valid
        _))
    (bind _returnvalue_2 (AddComponent|AddStaticMeshComponent false (Math|Transform|MakeTransform (Math|Vector|MakeVector (Math|Random|RandomFloatinRange _returnvalue _spawnradius) (Math|Random|RandomFloatinRange _returnvalue _spawnradius) (Math|Random|RandomFloatinRange _returnvalue _spawnradius)) (Math|Rotator|MakeRotator (Math|Random|RandomFloatinRange -1.8e+02 1.8e+02) (Math|Random|RandomFloatinRange -1.8e+02 1.8e+02) (Math|Random|RandomFloatinRange -1.8e+02 1.8e+02)) (* (Math|Random|RandomFloatinRange (Variables|Default|GetMaxScaleFactor) (+ 1.0 (Variables|Default|GetMaxScaleFactor))) "1.000000,1.000000,1.000000"))))
    (bind _output_get_2 (Variables|Default|SetStaticComponentReference _returnvalue_2))
    (Components|StaticMesh|SetStaticMesh _output_get_2 (Variables|Default|GetMesh))
    (for _array_element_2 (Variables|Default|GetSonoTraceUEActors)
      (Class|SonoTraceUEActor|AddActor _array_element_2 self))
    (Development|PrintString "Single object spawned!" true true "(R=1.000000,G=0.000000,B=0.688297,A=1.000000)" 1.0 "ObjectSingleSpawnerTest")
    (bind _output_get_3 (Variables|Default|SetSpawnCounter (+ (Variables|Default|GetSpawnCounter) 1)))
    (if (== _output_get_3 (Variables|Default|GetSpawnMaxTimes))
      (Actor|Tick|SetActorTickEnabled false)
      (Development|PrintString "Max single spawner objects reached" true true "(R=1.000000,G=0.000000,B=0.688297,A=1.000000)" 1.0 "ObjectSingleSpawnerTest"))))

(event EventBeginPlay
  (if (Variables|Default|GetEnable)
    (Actor|Tick|SetActorTickEnabled true)
    (bind _outactors (Actor|GetAllActorsOfClass "/Script/SonoTraceUE.SonoTraceUEActor"))
    (Variables|Default|SetSonoTraceUEActors _outactors)))

(fn ConstructionScript)