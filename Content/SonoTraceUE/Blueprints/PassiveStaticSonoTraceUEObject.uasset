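; SonoTraceUE actor that oscillates its child sensor and one of that sensor's receivers at runtime.
; BeginPlay sets the tick interval, caches the child sensor actor and reads the selected receiver's generated position.
; Each tick slides the sensor along relative Y via SetNewSensorRelativeTransform and the receiver along Z via SetNewReceiverPositions, without reapplying the offset.
; Each motion has its own speed and reverses direction when it reaches its symmetric limit.
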(event EventBeginPlay
  ;[1 1 1] set tick interval & retrieve one of the receiver positions
  (Actor|Tick|SetActorTickInterval (Variables|Default|GetTick%20Interval))
  (bind _assono_trace_ueactor (Utilities|Casting|CastToSonoTraceUEActor (Variables|/Script/Engine.ChildActorComponent|GetChildActor (Variables|Default|GetSonoTraceUESensorChildComponent))))
  (Variables|Default|SetSonoTraceUESensorActor _assono_trace_ueactor)
  (Variables|Default|SetReceiverPosition (Utilities|Array|Get(acopy) (.finalreceiverpositions (Variables|/Script/SonoTraceUE.SonoTraceUEActor|GetGeneratedSettings (Variables|Default|GetSonoTraceUESensorActor))) (Variables|Default|GetReceiverIndex))))

(event EventTick
  (params (DeltaSeconds :type Float%20%28single-precision%29))
  (bind _sonotraceuesensorchildcomponent (Variables|Default|GetSonoTraceUESensorChildComponent))
  (bind _relativelocation (Variables|/Script/Engine.SceneComponent|GetRelativeLocation _sonotraceuesensorchildcomponent))
  ;[1 1 1] On each tick move the sensor relative transform
  (Utilities|FlowControl|Sequence
    (:then_0
      (Class|SonoTraceUEActor|SetNewSensorRelativeTransform (Variables|Default|GetSonoTraceUESensorActor) (Math|Vector|MakeVector (.x _relativelocation) (+ (.y _relativelocation) (* (* DeltaSeconds (Variables|Default|GetSensorTranslationSpeed)) (Variables|Default|GetSensorTranslationDirection))) (.z _relativelocation)) (Variables|/Script/Engine.SceneComponent|GetRelativeRotation _sonotraceuesensorchildcomponent))
      (if (>= (Math|Float|Absolute(Float) (+ (.y _relativelocation) (* (* DeltaSeconds (Variables|Default|GetSensorTranslationSpeed)) (Variables|Default|GetSensorTranslationDirection)))) (Variables|Default|GetSensorMaximumYTranslation))
        (Variables|Default|SetSensorTranslationDirection (* (Variables|Default|GetSensorTranslationDirection) -1.0))))
    (:then_1
      ;[1 1 1] On tick move that one single receiver transform
      (bind _output_get (Variables|Default|SetReceiverPosition (Math|Vector|MakeVector (.x (Variables|Default|GetReceiverPosition)) (.y (Variables|Default|GetReceiverPosition)) (+ (.z (Variables|Default|GetReceiverPosition)) (* (* DeltaSeconds (Variables|Default|GetReceiverTranslationSpeed)) (Variables|Default|GetReceiverTranslationDirection))))))
      (Class|SonoTraceUEActor|SetNewReceiverPositions (Variables|Default|GetSonoTraceUESensorActor) (Utilities|Array|MakeArray (Variables|Default|GetReceiverIndex)) (Utilities|Array|MakeArray _output_get) false false)
      (if (>= (Math|Float|Absolute(Float) (+ (.z (Variables|Default|GetReceiverPosition)) (* (* DeltaSeconds (Variables|Default|GetReceiverTranslationSpeed)) (Variables|Default|GetReceiverTranslationDirection)))) (Variables|Default|GetReceiverMaximumZTranslation))
        (Variables|Default|SetReceiverTranslationDirection (* (Variables|Default|GetReceiverTranslationDirection) -1.0))))))

(fn ConstructionScript)