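; Test actor that exercises runtime adding and removing of static mesh components in SonoTraceUE.
; When enabled, it caches all SonoTraceUE actors on BeginPlay, then at a set rate randomly chooses to spawn or destroy.
; Spawns add a randomly transformed mesh component to itself, up to a maximum, and register it with every SonoTraceUE actor.
; Removals unregister a random component from those actors before destroying it, with each outcome printed on screen.
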(event EventTick
  (params (DeltaSeconds :type Float%20%28single-precision%29))
  (bind _spawnradius (Variables|Default|GetSpawnRadius))
  (bind _staticcomponents (Variables|Default|GetStaticComponents))
  (bind _returnvalue (* _spawnradius -1.0))
  (bind _output_get (Variables|Default|SetTimePassed (+ DeltaSeconds (Variables|Default|GetTimePassed))))
  (if (>= _output_get (/ 1.0 (Variables|Default|GetRate)))
    (Variables|Default|SetTimePassed 0.0)
    (if (Math|Random|RandomBoolwithWeight (/ (Variables|Default|GetSpawnChance) 1e+02))
      (if (< (Utilities|Array|Length (Variables|Default|GetStaticComponents)) (Variables|Default|GetSpawnMaxAmount))
        (bind _returnvalue_2 (AddComponent|AddStaticMeshComponent false (Math|Transform|MakeTransform (Math|Vector|MakeVector (Math|Random|RandomFloatinRange _returnvalue _spawnradius) (Math|Random|RandomFloatinRange _returnvalue _spawnradius) (Math|Random|RandomFloatinRange _returnvalue _spawnradius)) (Math|Rotator|MakeRotator (Math|Random|RandomFloatinRange -1.8e+02 1.8e+02) (Math|Random|RandomFloatinRange -1.8e+02 1.8e+02) (Math|Random|RandomFloatinRange -1.8e+02 1.8e+02)) (* (Math|Random|RandomFloatinRange (Variables|Default|GetMaxScaleFactor) (+ 1.0 (Variables|Default|GetMaxScaleFactor))) "1.000000,1.000000,1.000000"))))
        (Utilities|Array|Add (Variables|Default|GetStaticComponents) _returnvalue_2)
        (Components|StaticMesh|SetStaticMesh _returnvalue_2 (Variables|Default|GetMesh))
        (for _array_element (Variables|Default|GetSonoTraceUEActors)
          (Class|SonoTraceUEActor|AddStaticMeshComponent _array_element _returnvalue_2 (Utilities|String|ToString(Name) (Class|Actor|GetAttachParentSocketName))))
        (Development|PrintString "Multi object spawned!" true true "(R=0.000000,G=1.000000,B=0.000000,A=1.000000)" 1.0 "ObjectMultiSpawnerTest")
        (else
          (Development|PrintString "Could not spawn as maximum multi objects reached" true true "(R=0.000000,G=1.000000,B=0.000000,A=1.000000)" 1.0 "ObjectMultiSpawnerTest")))
      (elif (Utilities|Array|IsNotEmpty _staticcomponents)
        (bind _output_get_2 (Variables|Default|SetTempStaticRefToDelete (.OutItem (Utilities|Array|Random _staticcomponents))))
        (for _array_element_2 (Variables|Default|GetSonoTraceUEActors)
          (Class|SonoTraceUEActor|RemoveStaticMeshComponent _array_element_2 _output_get_2))
        (Utilities|Array|RemoveItem (Variables|Default|GetStaticComponents) _output_get_2)
        (Components|DestroyComponent _output_get_2)
        (Development|PrintString "Multi object destroyed!" true true "(R=0.000000,G=1.000000,B=0.000000,A=1.000000)" 1.0 "ObjectMultiSpawnerTest")
        (else
          (Development|PrintString "No multi object object to destoy" true true "(R=0.000000,G=1.000000,B=0.000000,A=1.000000)" 1.0 "ObjectMultiSpawnerTest"))))))

(event EventBeginPlay
  (if (Variables|Default|GetEnable)
    (Actor|Tick|SetActorTickEnabled true)
    (bind _outactors (Actor|GetAllActorsOfClass "/Script/SonoTraceUE.SonoTraceUEActor"))
    (Variables|Default|SetSonoTraceUEActors _outactors)))

(fn ConstructionScript)