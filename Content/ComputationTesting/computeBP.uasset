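; Benchmark Blueprint that stress-tests a child SonoTraceLab sensor actor across parameter ranges, saving results to file.
; After a five-second delay, Tick runs the selected test type: offline mesh preprocessing, ray tracing shader or simulation components.
; Successive ticks step through combinations of counts like triangles, rays, bounces, emitters, receivers and frequency bins as nested counters, disabling Tick at the limit.
; Simulation combinations failing the memory-limit estimate are skipped.
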(event EventBeginPlay
  ;[1 1 1] Init
  (bind _assono_trace_ueactor (Utilities|Casting|CastToSonoTraceUEActor (Variables|/Script/Engine.ChildActorComponent|GetChildActor (Variables|Components|GetSonoTraceLabSensorChildComponent))))
  (Variables|Default|SetSonoTraceLabSensorActor _assono_trace_ueactor)
  (Variables|MeshPreprocessingTest|SetcurrentTriangleValue (Variables|MeshPreprocessingTest|GetstartTriangleAmount))
  (Variables|SimulationTest|SetcurrentPointValue (Variables|SimulationTest|GetstartPointAmount))
  (Variables|Default|SetcurrentFrequencyBin (Variables|Default|GetstartFrequencyBins))
  (Variables|Default|SetcurrentBounce (Variables|Default|GetstartBounces))
  (Variables|Default|SetcurrentReceiverCount (Variables|Default|GetstartReceivers))
  (Variables|Default|SetcurrentEmitterCount (Variables|Default|GetstartEmitters))
  (Variables|RaytracingShaderTest|SetcurrentRayValue (Variables|RaytracingShaderTest|GetstartRayAmount)))

(event EventTick
  (params (DeltaSeconds :type Float%20%28single-precision%29))
  (bind _emitterpositions (Variables|Default|GetemitterPositions))
  (bind _receiverpositions (Variables|Default|GetreceiverPositions))
  (bind _emitterpositions_2 (Variables|Default|GetemitterPositions))
  (if (Variables|Default|Getinit)
    (switch Utilities|FlowControl|Switch|SwitchonESonoTraceUEDebugTestType (Variables|Default|Gettype)
      (:OfflineMeshPreprocessing
        ;[1 1 1] Mesh preprocessing tests
        (bind _output_get (Variables|MeshPreprocessingTest|SetcurrentTriangleValue (* (Variables|MeshPreprocessingTest|GettriangleMultiplier) (Variables|MeshPreprocessingTest|GetcurrentTriangleValue))))
        (bind _index (Utilities|StepforLoop (Variables|Default|GetstartFrequencyBins) (Variables|Default|GetmaxFrequencyBins) (Variables|Default|GetfrequencyBinsStep))
          (:LoopBody
            (for _index_2 (range 1 (Variables|Default|GetmaxRuns))
              (Class|SonoTraceUEActor|DebugRunMeshPreprocessingTest (Variables|Default|GetSonoTraceLabSensorActor) (Variables|MeshPreprocessingTest|GetcurrentTriangleValue) _index "Mesh Preprocessing Test" true "" true)))
          (:Completed
            (if (>= _output_get (Variables|MeshPreprocessingTest|GetmaxTriangleAmount))
              ;[1 1 1] Stop
              (Actor|Tick|SetActorTickEnabled false :!label _label)))))
      (:RayTracingShader
        ;[1 1 1] Raytracing tests
        (Utilities|Array|Clear _emitterpositions_2)
        (for _index_3 (range 0 (- (Variables|Default|GetcurrentEmitterCount) 1))
          (Utilities|Array|Add _emitterpositions_2 (Math|Vector|MakeVector 0.0 (Math|Conversions|ToFloat(Integer) _index_3) 0.0)))
        (bind _boutteststarted (Class|SonoTraceUEActor|DebugRunRaytracingShaderTest (Variables|Default|GetSonoTraceLabSensorActor) (Variables|Default|GetemitterPositions) (Variables|RaytracingShaderTest|GetcurrentRayValue) (Variables|Default|GetcurrentBounce) (Variables|Default|GetmaxRuns) "Ray Tracing Shader Test" true "" true))
        (if _boutteststarted
          (bind _output_get_2 (Variables|Default|SetcurrentBounce (+ (Variables|Default|GetcurrentBounce) (Variables|Default|GetbounceStep))))
          (if (> _output_get_2 (Variables|Default|GetmaxBounces))
            (Variables|Default|SetcurrentBounce (Variables|Default|GetstartBounces))
            (bind _output_get_3 (Variables|Default|SetcurrentEmitterCount (+ (Variables|Default|GetcurrentEmitterCount) (Variables|Default|GetEmittersStep))))
            (if (> _output_get_3 (Variables|Default|GetmaxEmitters))
              (Variables|Default|SetcurrentEmitterCount (Variables|Default|GetstartEmitters))
              (bind _output_get_4 (Variables|RaytracingShaderTest|SetcurrentRayValue (* (Variables|RaytracingShaderTest|GetrayMultiplier) (Variables|RaytracingShaderTest|GetcurrentRayValue))))
              (if (> _output_get_4 (Variables|RaytracingShaderTest|GetmaxRayAmount))
                (goto _label))))))
      (:SimulationComponents
        ;[1 1 1] Simulation tests
        (bind (_outestimatedmemorymb _outtotalestimatedmemorymb _returnvalue) (Class|SonoTraceUEActor|WouldSimulationTestFitinMemory (Variables|Default|GetSonoTraceLabSensorActor) (Variables|Default|GetcurrentEmitterCount) (Variables|Default|GetcurrentReceiverCount) (Variables|Default|GetcurrentFrequencyBin) (Variables|SimulationTest|GetcurrentPointValue) (Variables|Default|GetcurrentBounce) (Variables|SimulationTest|GetMemory%20Limit%20MB) true true true))
        (if _returnvalue
          (Utilities|Array|Clear _emitterpositions)
          (for _index_4 (range 0 (- (Variables|Default|GetcurrentEmitterCount) 1))
            (Utilities|Array|Add _emitterpositions (Math|Vector|MakeVector 0.0 (Math|Conversions|ToFloat(Integer) _index_4) 0.0)))
          (Utilities|Array|Clear _receiverpositions)
          (for _index_5 (range 0 (- (Variables|Default|GetcurrentReceiverCount) 1))
            (Utilities|Array|Add _receiverpositions (Math|Vector|MakeVector (Math|Conversions|ToFloat(Integer) _index_5) 0.0 0.0)))
          (Class|SonoTraceUEActor|DebugRunSimulationTest (Variables|Default|GetSonoTraceLabSensorActor) (Variables|SimulationTest|GetrunRayTracingParseTest) (Variables|SimulationTest|GetrunSpecularSimTest) (Variables|SimulationTest|GetrunDiffractionSimTest) (Variables|Default|GetemitterPositions) (Variables|Default|GetreceiverPositions) (Variables|SimulationTest|GetcurrentPointValue) (Variables|Default|GetcurrentBounce) (Variables|Default|GetcurrentFrequencyBin) (Variables|Default|GetmaxRuns) "Simulation Test" true "" true))
        (bind _output_get_5 (Variables|Default|SetcurrentFrequencyBin (+ (Variables|Default|GetcurrentFrequencyBin) (Variables|Default|GetfrequencyBinsStep))))
        (if (> _output_get_5 (Variables|Default|GetmaxFrequencyBins))
          (Variables|Default|SetcurrentFrequencyBin (Variables|Default|GetstartFrequencyBins))
          (bind _output_get_6 (Variables|Default|SetcurrentBounce (+ (Variables|Default|GetcurrentBounce) (Variables|Default|GetbounceStep))))
          (if (> _output_get_6 (Variables|Default|GetmaxBounces))
            (Variables|Default|SetcurrentBounce (Variables|Default|GetstartBounces))
            (bind _output_get_7 (Variables|Default|SetcurrentReceiverCount (* (Variables|Default|GetcurrentReceiverCount) (Variables|Default|GetreceiversMultiplier))))
            (if (> _output_get_7 (Variables|Default|GetmaxReceivers))
              (Variables|Default|SetcurrentReceiverCount (Variables|Default|GetstartReceivers))
              (bind _output_get_8 (Variables|Default|SetcurrentEmitterCount (+ (Variables|Default|GetcurrentEmitterCount) (Variables|Default|GetEmittersStep))))
              (if (> _output_get_8 (Variables|Default|GetmaxEmitters))
                (Variables|Default|SetcurrentEmitterCount (Variables|Default|GetstartEmitters))
                (bind _output_get_9 (Variables|SimulationTest|SetcurrentPointValue (* (Variables|SimulationTest|GetpointMultiplier) (Variables|SimulationTest|GetcurrentPointValue))))
                (if (> _output_get_9 (Variables|SimulationTest|GetmaxPointAmount))
                  (goto _label))))))))
    (else
      ;[1 1 1] Init
      (Utilities|FlowControl|DoOnce false
        (:Completed
          (Utilities|FlowControl|Delay 5.0)
          (Variables|Default|Setinit true))))))

(fn ConstructionScript)